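; BP_GameMode is the game mode for a turn-based game, containing only debug aids for the turn system.
; On BeginPlay it creates the DevWidget_ChangeTurn developer widget and adds it to the viewport.
; Every Tick it reads GameStateInstance and prints the current turn's display name and the turn count on screen, using zero-duration strings as a live readout.
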(event EventBeginPlay
  (bind _returnvalue (UserInterface|CreateWidget "/Game/Game/UI/Dev/DevWidget_ChangeTurn.DevWidget_ChangeTurn_C"))
  (UserInterface|Viewport|AddtoViewport _returnvalue 0))

(event EventTick
  (params (DeltaSeconds :type Float%20%28single-precision%29))
  (bind _gamestateinstance (Variables|Default|GetGameStateInstance))
  (bind _returnvalue (Class|DGameState|GetCurrentTurn _gamestateinstance))
  (Development|PrintString (Utilities|GetDisplayName _returnvalue) true true "(R=0.000000,G=0.660000,B=1.000000,A=1.000000)" 0.0)
  (Development|PrintString (Utilities|String|Append "Current Turn:" (Utilities|String|ToString(Integer) (Variables|/Script/FirstGameTurnBased.DGameState|GetTurnCount _gamestateinstance))) true true "(R=0.000000,G=0.660000,B=1.000000,A=1.000000)" 0.0))

(fn ConstructionScript)