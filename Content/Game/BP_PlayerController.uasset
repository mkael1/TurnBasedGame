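; Player controller that reacts to turn-based combat events from the game mode.
; On BeginPlay it binds to the combat-started and turn-changed delegates on DGameModeBase.
; When combat starts with the party leader as the player, it disables the leader's character movement and toggles the combat UI.
; Each turn change passes the active actor to SetActivePartyMember.
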(event Custom|OnTurnChanged_Event
  (params (Instigator :type Actor%20Object%20Reference) (ActiveActor :type Actor%20Object%20Reference) (TurnCount :type Integer))
  ;[1 1 1] On turn changed
  (Class|DPlayerController|SetActivePartyMember ActiveActor))

(event Custom|OnCombatStarted_Event
  (params (Player :type Actor%20Object%20Reference) (Enemy :type Actor%20Object%20Reference))
  ;[1 1 1] On Combat Begin
  (bind _returnvalue (Class|DPlayerController|GetPartyLeader))
  (if (== _returnvalue Player)
    (Pawn|Components|CharacterMovement|DisableMovement (.AsCharacter%20Movement%20Component (Utilities|Casting|CastToCharacterMovementComponent (Actor|GetComponentbyClass _returnvalue "/Script/Engine.MovementComponent"))))
    (Class|DPlayerController|ToggleCombatUI)))

(event EventBeginPlay
  (bind _returnvalue (Game|GetGameMode))
  (bind _asdgame_mode_base (Utilities|Casting|CastToDGameModeBase _returnvalue))
  (EventDispatchers|AssignOnCombatStarted _asdgame_mode_base (delegate Custom|OnCombatStarted_Event))
  (EventDispatchers|AssignOnTurnChanged _asdgame_mode_base (delegate Custom|OnTurnChanged_Event)))

(fn ConstructionScript)