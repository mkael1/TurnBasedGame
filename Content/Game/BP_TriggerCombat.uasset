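; BP_TriggerCombat is a trigger volume that starts combat when an actor overlaps it.
; On overlap it spawns an EnemyPawn with AI at EnemySpawnPoint, then calls EnterCombat on DGameModeBase with the overlapping actor and the new enemy.
; BeginPlay draws a long-lived debug box around the collision bounds.
; The overlapping actor is not filtered, and the node disabling collision is unconnected, so the trigger can fire repeatedly.
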(event EventBeginPlay
  (bind _collisioncomponent (Variables|Default|GetCollisionComponent))
  (bind (_origin _boxextent) (Collision|GetComponentBounds _collisioncomponent))
  (Rendering|Debug|DrawDebugBox :Center _origin :Extent _boxextent :Duration 1e+03))

(event Collision|EventActorBeginOverlap
  (params (OtherActor :type Actor%20Object%20Reference))
  (bind _returnvalue (AI|SpawnAIFromClass (Variables|Default|GetEnemyPawn) 0 (Transformation|GetWorldLocation (Variables|Default|GetEnemySpawnPoint)) "0, 0, 0" false 0))
  (Class|DGameModeBase|EnterCombat (.AsDGame%20Mode%20Base (Utilities|Casting|CastToDGameModeBase (Game|GetGameMode))) OtherActor _returnvalue))

(fn ConstructionScript)